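; Enemy actor that turns to face a seen third-person character (a class named NOT_IN_USE) and attempts to fire at it.
; Pawn sensing triggers spawning at the projectile point with a 0.2-second cooldown, but the spawn class is unset and the impulse is zero.
; BeginPlay caches three patrol points and picks one randomly.
; The timeline that would lerp between them never runs, so the enemy does not patrol.
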(event OnSeePawn(PawnSensing)
  (params (Pawn :type Pawn%20Object%20Reference))
  (bind _asnot_in_use_third_person_character (Utilities|Casting|CastToNOT_IN_USE_ThirdPersonCharacter Pawn))
  (Utilities|FlowControl|Sequence
    (:then_0
      (Transformation|SetActorRotation (Math|Rotator|FindLookatRotation (Transformation|GetActorLocation) (Transformation|GetActorLocation _asnot_in_use_third_person_character))))
    (:then_1
      (if (Variables|Default|GetSpawnProjectile)
        (bind _returnvalue (Game|SpawnActorfromClass 0 (Transformation|GetWorldTransform (Variables|Default|GetProjectilespawnLocation)) "Undefined" 0 0))
        (Physics|AddImpulse (Variables|Default|GetCollisionComponent _returnvalue) "0, 0, 0" "None" false)
        (Variables|Default|SetSpawnProjectile false)
        (Utilities|FlowControl|Delay 0.2)
        (Variables|Default|SetSpawnProjectile true)))))

(event EventBeginPlay
  (Variables|Default|SetPatrolPoints (Utilities|Array|MakeArray (Transformation|GetWorldLocation (Variables|Default|GetMovePosition1)) (Transformation|GetWorldLocation (Variables|Default|GetMovePosition2)) (Transformation|GetWorldLocation (Variables|Default|GetMovePosition3))))
  (CallFunction|GetRandomLocation))

(fn ConstructionScript)

(fn GetRandomLocation
  (Variables|Default|SetCurrentPatrolPoint (Math|Random|RandomInteger (Utilities|Array|Length (Variables|Default|GetPatrolPoints)))))