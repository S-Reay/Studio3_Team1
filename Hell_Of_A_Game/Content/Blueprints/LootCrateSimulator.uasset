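; Loot crate simulator actor that rolls a random weapon drop once on BeginPlay and reports it through debug Print String messages.
; Three chained random-integer switches pick weapon type, skin color and effect with equal odds, each branch converging into the next roll.
; The results are appended into a reward message, with red error prints on each switch's default case.
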(event EventBeginPlay
  (Development|PrintString "Opening Crate" true true "(R=0.000000,G=0.660000,B=1.000000,A=1.000000)" 2e+01)
  (switch int (Math|Random|RandomIntegerinRange 0 2)
    (:Default
      (Development|PrintString "Error  in Weapon Type" true true "(R=1.000000,G=0.000000,B=0.021336,A=1.000000)"))
    (:0
      (Variables|Default|SetWeaponType "Sword")
      (switch int (Math|Random|RandomIntegerinRange 0 4) :!label _label
        (:Default
          (Development|PrintString "Error in Skins" true true "(R=1.000000,G=0.000000,B=0.021336,A=1.000000)"))
        (:0
          (Variables|Default|SetSkin "Red")
          (switch int (Math|Random|RandomIntegerinRange 0 3) :!label _label_2
            (:Default
              (Development|PrintString "Error in Effect" true true "(R=1.000000,G=0.000000,B=0.021336,A=1.000000)"))
            (:0
              (Variables|Default|SetEffect "Charged")
              (Development|PrintString (Utilities|String|Append "Player received a " (Variables|Default|GetEffect) " " (Variables|Default|GetSkin) " " (Variables|Default|GetWeaponType)) true true "(R=0.346934,G=1.000000,B=0.000000,A=1.000000)" 2e+01 :!label _label_3))
            (:1
              (Variables|Default|SetEffect "Holy")
              (goto _label_3))
            (:2
              (Variables|Default|SetEffect "Cosmic")
              (goto _label_3))
            (:3
              (Variables|Default|SetEffect "Scorching")
              (goto _label_3))))
        (:1
          (Variables|Default|SetSkin "Green")
          (goto _label_2))
        (:2
          (Variables|Default|SetSkin "Blue")
          (goto _label_2))
        (:3
          (Variables|Default|SetSkin "White")
          (goto _label_2))
        (:4
          (Variables|Default|SetSkin "Black")
          (goto _label_2))))
    (:1
      (Variables|Default|SetWeaponType "Axe")
      (goto _label))
    (:2
      (Variables|Default|SetWeaponType "Dagger")
      (goto _label))))

(event Collision|EventActorBeginOverlap
  (params (OtherActor :type Actor%20Object%20Reference)))

(event EventTick
  (params (DeltaSeconds :type Float%20%28single-precision%29)))

(fn ConstructionScript)