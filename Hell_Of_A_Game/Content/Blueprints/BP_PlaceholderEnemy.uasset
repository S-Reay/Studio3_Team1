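; BP_PlaceholderEnemy is a stand-in enemy character that takes damage and dies.
; TakeDamage subtracts the damage from Health and, at zero or below, prints "Dead" and calls Ragdoll.
; Ragdoll turns on physics simulation for the mesh and disables character movement, leaving the capsule untouched.
; The construction script is empty.
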(event Custom|TakeDamage
  (params (Damage :type Integer))
  (Variables|Default|SetHealth (- (Variables|Default|GetHealth) Damage))
  (if (<= (Variables|Default|GetHealth) 0)
    (Development|PrintString "Dead")
    (CallFunction|Ragdoll)))

(fn ConstructionScript)

(fn Ragdoll
  (Physics|SetSimulatePhysics (Variables|Character|GetMesh) true)
  (Pawn|Components|CharacterMovement|DisableMovement (Variables|Character|GetCharacterMovement)))